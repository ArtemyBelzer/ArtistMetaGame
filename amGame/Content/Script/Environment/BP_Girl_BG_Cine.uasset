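; BP_Girl_BG_Cine is a background girl character that can optionally walk to a path node and disappear.
; When GoToPaths is set, BeginPlay waits out a delay, spawns and possesses an AIController, then moves toward the first BackgroundCharacterPathnode found in the level.
; It snaps rotation once to face that node, and Tick destroys the actor when it gets close to it.
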(event `self.ReceiveBeginPlay`
  (if (`self.bGoToPaths`)
    (`KismetSystemLibrary.Delay` 9.0)
    (bind _returnvalue (`|SpawnActorFromClass` "/Script/AIModule.AIController" (`KismetMathLibrary.MakeTransform` (0.0 0.0 0.0)) "Undefined" "OverrideRootScale" null null))
    (`Controller.Possess` _returnvalue self)
    (bind _outactors (`GameplayStatics.GetAllActorsOfClass` "/Game/Script/Environment/BackgroundCharacterPathnode.BackgroundCharacterPathnode_C"))
    (bind _output_get (set `self.Path` _outactors))
    (bind _output_get_2 (set `self.Target` (`|GetArrayItem` _output_get)))
    (`AIController.MoveToActor` (`AIBlueprintHelperLibrary.GetAIController` self) _output_get_2 -1.0 true true true "/Game/Script/Environment/DefaultNavData.DefaultNavData_C" true)
    (`self.K2_SetActorRotation` (`KismetMathLibrary.Conv_VectorToRotator` (`KismetMathLibrary.Normal` (- (`self.K2_GetActorLocation` _output_get_2) (`self.K2_GetActorLocation`)))))))

(event `self.ReceiveTick`
  (params (DeltaSeconds :type "Float (single-precision)"))
  (if (`self.bGoToPaths`)
    (`/Engine/EditorBlueprintResources/StandardMacros.IsValid` (`self.Target`)
      (:`Is Valid`
        (if (< (`KismetMathLibrary.Vector_Distance` (`self.K2_GetActorLocation` (`self.Target`)) (`self.K2_GetActorLocation`)) 100.0)
          (`self.K2_DestroyActor`))))))

(fn `UserConstructionScript`)