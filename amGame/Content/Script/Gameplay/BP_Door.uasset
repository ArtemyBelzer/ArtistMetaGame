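; BP_Door is a locked door that opens once, when its matching possessible key item overlaps its key collision.
; It checks that the item's key target message returns this door, then plays a slowed timeline that drives the Arrow component's yaw.
; The key item is then unpossessed and teleported to the origin, and a flag blocks further triggers.
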(event `OpenDoor`
  (`TimelineComponent.SetPlayRate` (`self.DoorAnim`) 0.1)
  (bind (_direction _actorrot) (`Timeline|DoorAnim`)
    (:`Update`
      (`SceneComponent.K2_SetRelativeRotation` (`self.Arrow`) (`KismetMathLibrary.MakeRotator` 0.0 0.0 (* _actorrot 1.0)) false false))))

(event `self.KeyCollision.OnComponentBeginOverlap`
  (params (OverlappedComponent :type "PrimitiveComponent Object Reference") (OtherActor :type "Actor Object Reference") (OtherComp :type "PrimitiveComponent Object Reference") (OtherBodyIndex :type Integer) (bFromSweep :type Boolean) (SweepResult :type "HitResult Structure (by ref)"))
  (bind _setkey (`self.SetKey`))
  (if (`self.bDoorOpened`)
    _
    (elif (`KismetMathLibrary.ClassIsChildOf` (`GameplayStatics.GetObjectClass` OtherActor) "/Game/Script/Gameplay/PossessibleItem.PossessibleItem_C")
      (set `self.SetKey` OtherActor)
      (bind _target (message `/Game/Player/BPI_Player.GetKeyTarget` OtherActor))
      (if (== _target self)
        (`self.OpenDoor`)
        (set `self.bDoorOpened` true)
        (bind _aspossessible_item (cast `/Game/Script/Gameplay/PossessibleItem` _setkey))
        (`/Game/Script/Gameplay/PossessibleItem.UnpossesItem` _aspossessible_item)
        (`self.K2_SetActorLocation` _setkey (0.0 0.0 0.0) false true)))))

(fn `UserConstructionScript`)