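; BP_Stoplight is a traffic-light obstacle that a matching possessable key item opens once.
; Key collision overlap accepts a PossessibleItem whose key-target interface message returns this actor, then unpossesses it and teleports it to the world origin.
; Opening plays crash and explosion sounds while a timeline rolls the Arrow and disables Box collision.
; The stoplight destroys itself shortly after the animation finishes.
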(event `self.OpenDoor`
  (`/Engine/EditorBlueprintResources/StandardMacros.DoOnce` false
    (:`Completed`
      (`TimelineComponent.SetPlayRate` (`self.Timeline_0`) 0.25)
      (`GameplayStatics.SpawnSoundAtLocation` "/Game/Audio/SFX/box_crushes_traffic_light_Cue.box_crushes_traffic_light_Cue" (`self.K2_GetActorLocation`) (struct) 1.0 1.0 0.0 null null)
      (`GameplayStatics.PlaySoundAtLocation` "/Game/Audio/SFX/Explosion02.Explosion02" (`self.K2_GetActorLocation`) (struct) 1.0 1.0 0.0 null null null)
      (bind (_direction _actorrot) (`Timeline|Timeline_0`)
        (:`Update`
          (`SceneComponent.K2_SetRelativeRotation` (`self.Arrow`) (`KismetMathLibrary.MakeRotator` _actorrot) false false)
          (`PrimitiveComponent.SetCollisionEnabled` (`self.Box`) "NoCollision"))
        (:`Finished`
          (`KismetSystemLibrary.Delay` 1.0)
          (`self.K2_DestroyActor`))))))

(event `self.KeyCollision.OnComponentBeginOverlap`
  (params (OverlappedComponent :type "PrimitiveComponent Object Reference") (OtherActor :type "Actor Object Reference") (OtherComp :type "PrimitiveComponent Object Reference") (OtherBodyIndex :type Integer) (bFromSweep :type Boolean) (SweepResult :type "HitResult Structure (by ref)"))
  (bind _setkey (`self.SetKey`))
  (if (`self.bDoorOpened`)
    _
    (elif (`KismetMathLibrary.ClassIsChildOf` (`GameplayStatics.GetObjectClass` OtherActor) "/Game/Script/Gameplay/PossessibleItem.PossessibleItem_C")
      (set `self.SetKey` OtherActor)
      (bind _target (message `/Game/Player/BPI_Player.GetKeyTarget` OtherActor))
      (if (== _target self)
        (`self.OpenDoor`)
        (set `self.bDoorOpened` true)
        (bind _aspossessible_item (cast `/Game/Script/Gameplay/PossessibleItem` _setkey))
        (`/Game/Script/Gameplay/PossessibleItem.UnpossesItem` _aspossessible_item)
        (`self.K2_SetActorLocation` _setkey (0.0 0.0 0.0) false true)))))

(fn `UserConstructionScript`)