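; Game instance Blueprint that owns the single-slot save game, built on a DataStore save object.
; LoadSaveGame loads or creates the save and caches its data, while getters and SetCheckpoint forward to it through message calls.
; NewGameSaveRequest prompts before losing existing progress, and NewGameSavePermit deletes and recreates the slot.
; ContinueGameRequest always returns false, and the FadeSystem and LoadMenu events are empty.
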(event `self.FadeSystem`)

(event `self.LoadSaveGame`
  (`self.InitializeSaveGame`))

(event `self.LoadMenu`)

(event `/Game/Script/Core/BPI_Core.NewGameSavePermit`
  (`self.Create New Save Game`))

(fn `ContinueGameRequest`
  (returns (bSuccess :type Boolean))
  (return false))

(fn `Create New Save Game`
  (`GameplayStatics.DeleteGameInSlot` "SAV")
  (bind _returnvalue (`GameplayStatics.CreateSaveGameObject` "/Game/Script/Core/DataStore.DataStore_C"))
  (bind _output_get (set `self.SaveGame` _returnvalue))
  (bind _out (message `/Game/Script/Core/BPI_DataStore.GetSaveData` _output_get))
  (set `self.StoredSaveData` _out)
  (`GameplayStatics.SaveGameToSlot` (`self.SaveGame`) "SAV"))

(fn `GetSaveData`
  (returns (Out :type "/Game/Script/Core/GameData Structure"))
  (bind _out (message `/Game/Script/Core/BPI_DataStore.GetSaveData` (`self.SaveGame`)))
  (return _out))

(fn `GetSaveInitStatus`
  (returns (bIntialized :type Boolean))
  (bind _bintialized (message `/Game/Script/Core/BPI_DataStore.GetSaveInitStatus` (`self.SaveGame`)))
  (return _bintialized))

(fn `InitializeSaveGame`
  (bind _savegame (`self.SaveGame`))
  (bind _returnvalue (`GameplayStatics.DoesSaveGameExist` "SAV"))
  (if _returnvalue
    (bind _returnvalue_2 (`GameplayStatics.LoadGameFromSlot` "SAV"))
    (set `self.SaveGame` _returnvalue_2)
    (bind _out (message `/Game/Script/Core/BPI_DataStore.GetSaveData` _savegame))
    (set `self.StoredSaveData` _out)
    (else
      (bind _returnvalue_3 (`GameplayStatics.CreateSaveGameObject` "/Game/Script/Core/DataStore.DataStore_C"))
      (set `self.SaveGame` _returnvalue_3)
      (bind _out_2 (message `/Game/Script/Core/BPI_DataStore.GetSaveData` _savegame))
      (set `self.StoredSaveData` _out_2)
      (`GameplayStatics.SaveGameToSlot` (`self.SaveGame`) "SAV"))))

(fn `NewGameSaveRequest`
  (params (Instigator :type "Object Object Reference"))
  (returns (bSuccess :type Boolean) (Insitigator :type "Object Object Reference"))
  (bind _returnvalue (`GameplayStatics.DoesSaveGameExist` "SAV"))
  (if _returnvalue
    (`/Game/Script/UI/BPFL_UI.ShowMessagePrompt` Instigator "Are you sure you want to start a new game? You will lose your progress!" "NewEnumerator2" "NewEnumerator1")
    (return false null)))

(fn `SetCheckpoint`
  (params (Checkpoint :type Name) (Weight :type Integer))
  (returns (bSuccess :type Boolean))
  (bind _bsuccess (message `/Game/Script/Core/BPI_DataStore.SetCheckpoint` (`self.SaveGame`) Checkpoint Weight))
  (return _bsuccess))